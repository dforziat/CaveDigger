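; Game mode Blueprint for CaveDigger that runs the intro sequence, HUD and on-screen game timer.
; CreateHUD shows the intro widget and plays its flash animation.
; When that finishes, it swaps in the main HUD, starts the level music and calls StartGameTimer.
; Once the HUD exists, Tick calls UpdateScore, which, despite its name, writes the remaining game time to the HUD's timer text.
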(event Custom|Create%20HUD
  (bind _returnvalue (UserInterface|CreateWidget "/Game/UI/BPW_Intro.BPW_Intro_C"))
  (bind _output_get (Variables|Default|SetIntroWidget _returnvalue))
  (UserInterface|Viewport|AddtoViewport _returnvalue 0)
  (Components|Animation|PlayAnimation (Variables|Default|GetIntroWidget) (Variables|/Game/UI/BPW_Intro.BPW_Intro_C|GetIntroFlashAnimation _returnvalue) 0.0
    (:Finished
      (bind _returnvalue_2 (UserInterface|CreateWidget "/Game/UI/BPW_UI.BPW_UI_C"))
      (bind _output_get_2 (Variables|Default|SetHUD _returnvalue_2))
      (UserInterface|Viewport|AddtoViewport _output_get_2 0)
      (Widget|RemovefromParent (Variables|Default|GetIntroWidget))
      (Widget|SetVisibility (Variables|Default|GetHUD) "Visible")
      (Variables|Default|SetIsHUDCreated true)
      (Audio|PlaySound2D "/Game/Music/SC_LevelMusic.SC_LevelMusic" 1.0 1.0 0.0 0 0)
      (Class|CaveDiggerGameModeBase|StartGameTimer))))

(event EventBeginPlay)

(event EventTick
  (params (DeltaSeconds :type Float%20%28single-precision%29))
  (if (Variables|Default|GetIsHUDCreated)
    (CallFunction|UpdateScore)))

(fn ConstructionScript)

(fn UpdateScore
  (bind _returnvalue (Class|CaveDiggerGameModeBase|GetGameTimeRemaing))
  (Variables|/Script/UMG.TextBlock|SetText (Variables|/Game/UI/BPW_UI.BPW_UI_C|GetTimer (Variables|Default|GetHUD)) (Utilities|Text|ToText(Integer) _returnvalue)))