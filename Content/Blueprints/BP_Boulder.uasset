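; BP_Boulder is a physical boulder that damages dirt and the digger character when it hits them while moving.
; Component hit events act only above a small velocity threshold.
; Dirt hits apply dig damage, rate-limited by a CanHit flag that a timer resets.
; Hitting a digger deals damage, plays a crush sound and Niagara effect, then destroys the boulder.
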(event Custom|OnComponentHit_Event
  (params (HitComponent :type Primitive%20Component%20Object%20Reference) (OtherActor :type Actor%20Object%20Reference) (OtherComp :type Primitive%20Component%20Object%20Reference) (NormalImpulse :type Vector) (Hit :type Hit%20Result%20Structure%20%28by%20ref%29))
  (bind _returnvalue (Transformation|GetActorLocation))
  (if (> (Math|Vector|VectorLength (Transformation|GetComponentVelocity (Variables|Default|GetStaticMeshComp))) 5.0)
    (Utilities|FlowControl|Sequence
      (:then_0
        (bind _asdirt_parent (Utilities|Casting|CastToDirtParent OtherActor))
        (if (Variables|Default|GetCanHit)
          (Class|DirtParent|TakeDigDamage _asdirt_parent)
          (Variables|Default|SetCanHit false)
          (Utilities|Time|SetTimerbyEvent (delegate Custom|ResetCanHit) 1.5)))
      (:then_1
        (bind _asbp_digger_character (Utilities|Casting|CastToBP_DiggerCharacter OtherActor))
        (Class|DiggerCharacter|RecieveDamage _asbp_digger_character 1 _returnvalue)
        (Audio|PlaySoundatLocation "/Game/Sounds/Crush.Crush" _returnvalue "0, 0, 0" 1.0 1.0 0.0 0 0 0 0)
        (Niagara|SpawnSystematLocation "/Game/Particles/BoulderEmitter.BoulderEmitter" _returnvalue)
        (Actor|DestroyActor)))))

(event Custom|ResetCanHit
  (Variables|Default|SetCanHit true))

(event EventBeginPlay
  (Collision|AssignOnComponentHit (Variables|Default|GetStaticMeshComp) (delegate Custom|OnComponentHit_Event)))

(event Collision|EventActorBeginOverlap
  (params (OtherActor :type Actor%20Object%20Reference)))

(event EventTick
  (params (DeltaSeconds :type Float%20%28single-precision%29)))

(fn ConstructionScript)