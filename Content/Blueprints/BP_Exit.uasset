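; BP_Exit is the level exit in a cave-digging game, winning the game when the player reaches it.
; On BeginPlay it runs a box trace around its static mesh and destroys every hit actor tagged Dirt, with persistent debug drawing left on.
; When a BP_DiggerCharacter overlaps its Box component, it calls GameWin on BP_CaveDiggerGameModeBase.
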(event OnComponentBeginOverlap(Box)
  (params (OverlappedComponent :type Primitive%20Component%20Object%20Reference) (OtherActor :type Actor%20Object%20Reference) (OtherComp :type Primitive%20Component%20Object%20Reference) (OtherBodyIndex :type Integer) (bFromSweep :type Boolean) (SweepResult :type Hit%20Result%20Structure%20%28by%20ref%29))
  (Utilities|Casting|CastToBP_DiggerCharacter OtherActor)
  (bind _asbp_cave_digger_game_mode_base (Utilities|Casting|CastToBP_CaveDiggerGameModeBase (Game|GetGameMode)))
  (Class|CaveDiggerGameModeBase|GameWin _asbp_cave_digger_game_mode_base))

(event EventBeginPlay
  (CallFunction|DestroySurroundingDirt))

(event Collision|EventActorBeginOverlap
  (params (OtherActor :type Actor%20Object%20Reference)))

(event EventTick
  (params (DeltaSeconds :type Float%20%28single-precision%29)))

(fn ConstructionScript)

(fn DestroySurroundingDirt
  (bind _staticmesh (Variables|Default|GetStaticMesh))
  (bind _returnvalue (Transformation|GetWorldLocation _staticmesh))
  (bind _returnvalue_2 (+ _returnvalue "0.000000,40.000000,80.000000"))
  (bind (_outhits _returnvalue_3) (Class|KismetSystemLibrary|BoxTraceMulti _returnvalue_2 _returnvalue_2 "100.000000,100.000000,110.000000" "0, 0, 0" "TraceTypeQuery1" false 0 "Persistent" true))
  (if _returnvalue_3
    (for _array_element _outhits
      (if (Actor|ActorHasTag (.HitActor (Collision|BreakHitResult _array_element)) "Dirt")
        (Actor|DestroyActor (.HitActor (Collision|BreakHitResult _array_element)))))))